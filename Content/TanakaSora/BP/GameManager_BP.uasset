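; GameManager tracks the loop count for a corridor anomaly-spotting game.
; OnEntry increments LoopCount without an anomaly and resets it with one; OnExit does the reverse, and both print a debug string.
; SpawnCorridor loads a level instance by fixed name, and ChooseCorridor only fetches CorridorTable row names, with selection unfinished.
; Nothing here calls either function or sets HasAnomaly.
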(event `self.ReceiveBeginPlay`)

(event `OnEntry`
  (if (`self.bHasAnomaly`)
    (set `self.LoopCount` 0)
    (else
      (`/Engine/EditorBlueprintResources/StandardMacros.IncrementInt` (`self.LoopCount`)
        (:`  `
          _))))
  (`KismetSystemLibrary.PrintString` "Entry"))

(event `OnExit`
  (if (`self.bHasAnomaly`)
    (`/Engine/EditorBlueprintResources/StandardMacros.IncrementInt` (`self.LoopCount`)
      (:`  `
        _))
    (else
      (set `self.LoopCount` 0)))
  (`KismetSystemLibrary.PrintString` "Exit"))

(fn `ChooseCorridor`
  (`DataTableFunctionLibrary.GetDataTableRowNames` (`self.CorridorTable`)))

(fn `SpawnCorridor`
  (`LevelStreamingDynamic.LoadLevelInstance` "StreamingLevel" (0.0 0.0 0.0) (struct) "" null))

(fn `UserConstructionScript`)